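; Destructible wall Blueprint that reacts to explosions and can drop a power-up.
; When a Pwn_Explosion overlaps it, it fires its radial force impulse, runs the power-up roll, then destroys the overlapping explosion actor, not itself.
; The roll has a 30% chance to spawn a Pwn_PowerUp slightly above the wall's scene component, ignoring collisions.
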(event `self.ReceiveActorBeginOverlap`
  (params (OtherActor :type "Actor Object Reference"))
  ;[1 1 1] If explosion detected, break wall, spawn powerUP and destroy self
  (cast `/Game/Scripts_And_BP/Bomb/Pwn_Explosion` OtherActor)
  (`RadialForceComponent.FireImpulse` (`self.RadialForce`))
  (`self.Spawn_PowerUp`)
  (`self.K2_DestroyActor` OtherActor))

(fn `Spawn_PowerUp`
  ;[1 1 1] Spawn powerup on wall location
  ;;[1 1 1] Needed over 70 (30%) to spawn PowerUp
  (if (>= (`KismetMathLibrary.RandomInteger` 100) 70)
    (`|SpawnActorFromClass` "/Game/Scripts_And_BP/PowerUps/Pwn_PowerUp.Pwn_PowerUp_C" (`KismetMathLibrary.MakeTransform` (`KismetMathLibrary.MakeVector` (.x (`SceneComponent.K2_GetComponentLocation` (`self.Scene`))) (.y (`SceneComponent.K2_GetComponentLocation` (`self.Scene`))) (+ (.z (`SceneComponent.K2_GetComponentLocation` (`self.Scene`))) 60.0))) "AlwaysSpawn" "OverrideRootScale" null null)))

(fn `UserConstructionScript`)