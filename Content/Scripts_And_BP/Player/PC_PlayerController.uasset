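; Player controller that routes input for two local players in a bomb-placing game and handles round restarts.
; Separate move and bomb mappings per player are forwarded as messages to the Pawn_Player at player index 1 or 2.
; Restart input stays in the controller so it still works when both players die.
; When RoundEnd is set, it clears the flag and calls RestartMap on the first CameraActor_Blueprint found.
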(event `InputAxis|MoveUp1`
  (params (AxisValue :type "Float (single-precision)"))
  ;[1 1 1] Send MoveUpRight Commands
  (bind _aspawn_player (cast `/Game/Scripts_And_BP/Player/Pawn_Player` (`GameplayStatics.GetPlayerPawn` 1)))
  (message `/Game/Scripts_And_BP/Player/I_PlayerCalls.MoveUpDown` _aspawn_player AxisValue))

(event `InputAction|PlaceBomb1`
  (params (Key :type "Key Structure"))
  ;[1 1 1] Send Set Bombs Command
  (:`Pressed`
    (bind _aspawn_player (cast `/Game/Scripts_And_BP/Player/Pawn_Player` (`GameplayStatics.GetPlayerPawn` 1)))
    (message `/Game/Scripts_And_BP/Player/I_PlayerCalls.PlaceBomb` _aspawn_player)))

(event `InputAction|PlaceBomb2`
  (params (Key :type "Key Structure"))
  ;[1 1 1] Send Set Bombs Command
  (:`Pressed`
    (bind _aspawn_player (cast `/Game/Scripts_And_BP/Player/Pawn_Player` (`GameplayStatics.GetPlayerPawn` 2)))
    (message `/Game/Scripts_And_BP/Player/I_PlayerCalls.PlaceBomb` _aspawn_player)))

(event `InputAxis|MoveUp2`
  (params (AxisValue :type "Float (single-precision)"))
  ;[1 1 1] Send MoveUpRight Commands
  (bind _aspawn_player (cast `/Game/Scripts_And_BP/Player/Pawn_Player` (`GameplayStatics.GetPlayerPawn` 2)))
  (message `/Game/Scripts_And_BP/Player/I_PlayerCalls.MoveUpDown` _aspawn_player AxisValue))

(event `InputAction|RestartGame`
  (params (Key :type "Key Structure"))
  ;[1 1 1] Restart Game (this one remains in here, if is sent to players and both die there will be no way to restart game
  (:`Pressed`
    (if (`self.RoundEnd`)
      (set `self.RoundEnd` false)
      (bind _outactors (`GameplayStatics.GetAllActorsOfClass` "/Game/Scripts_And_BP/CameraPlayer/CameraActor_Blueprint.CameraActor_Blueprint_C"))
      (`/Game/Scripts_And_BP/CameraPlayer/CameraActor_Blueprint.RestartMap` (`|GetArrayItem` _outactors)))))

(event `InputAxis|MoveRight1`
  (params (AxisValue :type "Float (single-precision)"))
  ;[1 1 1] Send Move RightLeft Commands
  (bind _aspawn_player (cast `/Game/Scripts_And_BP/Player/Pawn_Player` (`GameplayStatics.GetPlayerPawn` 1)))
  (message `/Game/Scripts_And_BP/Player/I_PlayerCalls.MoveRightLeft` _aspawn_player AxisValue))

(event `InputAxis|MoveRight2`
  (params (AxisValue :type "Float (single-precision)"))
  ;[1 1 1] Send Move RightLeft Commands
  (bind _aspawn_player (cast `/Game/Scripts_And_BP/Player/Pawn_Player` (`GameplayStatics.GetPlayerPawn` 2)))
  (message `/Game/Scripts_And_BP/Player/I_PlayerCalls.MoveRightLeft` _aspawn_player AxisValue))

(fn `UserConstructionScript`)